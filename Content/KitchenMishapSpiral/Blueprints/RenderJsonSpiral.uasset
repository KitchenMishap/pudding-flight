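; Actor that renders a spiral from a JSON file as instanced meshes on two HismForSpiral child actors.
; BuildRenderedJson turns the JSON path and asset limit into two transform sets, plus colours and opacities.
; Separate functions add instances with a shared material, batch-update their transforms, or clear them.
; A colour pass writes RGB and opacity into per-instance custom data, on the first child's HISM only.
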(event EventBeginPlay)

(event Collision|EventActorBeginOverlap
  (params (OtherActor :type Actor%20Object%20Reference)))

(event EventTick
  (params (DeltaSeconds :type Float%20%28single-precision%29)))

(fn ConstructionScript)

(fn LoadSpiralWithoutColours
  (bind _material (Variables|Default|GetMaterial))
  (bind _ashism_for_spiral (Utilities|Casting|CastToHismForSpiral (Variables|/Script/Engine.ChildActorComponent|GetChildActor (Variables|Default|GetExampleDaySpiral))))
  (Default|SetMaterial _ashism_for_spiral _material)
  (bind _ashism_for_spiral_2 (Utilities|Casting|CastToHismForSpiral (Variables|/Script/Engine.ChildActorComponent|GetChildActor (Variables|Default|GetExampleDaySpiral1))))
  (Default|SetMaterial _ashism_for_spiral_2 _material)
  (bind (_colours _opacities _hism2transforms _returnvalue) (CallFunction|BuildRenderedJson "0.000000,0.000000,50.000000" 1e+02 (Variables|Default|GetJsonPath) (Variables|Default|GetMaxAssets)))
  (Components|InstancedStaticMesh|AddInstances (Variables|/Game/KitchenMishapSpiral/Blueprints/HismForSpiral.HismForSpiral_C|GetHierarchicalInstancedStaticMesh _ashism_for_spiral) _returnvalue false false true)
  (Components|InstancedStaticMesh|AddInstances (Variables|/Game/KitchenMishapSpiral/Blueprints/HismForSpiral.HismForSpiral_C|GetHierarchicalInstancedStaticMesh _ashism_for_spiral_2) _hism2transforms false false true))

(fn DestroySpiral
  (bind _ashism_for_spiral (Utilities|Casting|CastToHismForSpiral (Variables|/Script/Engine.ChildActorComponent|GetChildActor (Variables|Default|GetExampleDaySpiral))))
  (bind _ashism_for_spiral_2 (Utilities|Casting|CastToHismForSpiral (Variables|/Script/Engine.ChildActorComponent|GetChildActor (Variables|Default|GetExampleDaySpiral1))))
  (Components|InstancedStaticMesh|ClearInstances (Variables|/Game/KitchenMishapSpiral/Blueprints/HismForSpiral.HismForSpiral_C|GetHierarchicalInstancedStaticMesh _ashism_for_spiral))
  (Components|InstancedStaticMesh|ClearInstances (Variables|/Game/KitchenMishapSpiral/Blueprints/HismForSpiral.HismForSpiral_C|GetHierarchicalInstancedStaticMesh _ashism_for_spiral_2)))

(fn LoadSpiralColours
  (bind _ashism_for_spiral (Utilities|Casting|CastToHismForSpiral (Variables|/Script/Engine.ChildActorComponent|GetChildActor (Variables|Default|GetExampleDaySpiral))))
  (bind (_colours _opacities _hism2transforms _returnvalue) (CallFunction|BuildRenderedJson "0.000000,0.000000,50.000000" 1e+02 (Variables|Default|GetJsonPath) (Variables|Default|GetMaxAssets)))
  (for (_ _array_index) _returnvalue
    (Components|InstancedStaticMesh|SetCustomDataValue (Variables|/Game/KitchenMishapSpiral/Blueprints/HismForSpiral.HismForSpiral_C|GetHierarchicalInstancedStaticMesh _ashism_for_spiral) _array_index 0 (.X (Math|Vector|BreakVector (Utilities|Array|Get(acopy) _colours _array_index))) true)
    (Components|InstancedStaticMesh|SetCustomDataValue (Variables|/Game/KitchenMishapSpiral/Blueprints/HismForSpiral.HismForSpiral_C|GetHierarchicalInstancedStaticMesh _ashism_for_spiral) _array_index 1 (.Y (Math|Vector|BreakVector (Utilities|Array|Get(acopy) _colours _array_index))) true)
    (Components|InstancedStaticMesh|SetCustomDataValue (Variables|/Game/KitchenMishapSpiral/Blueprints/HismForSpiral.HismForSpiral_C|GetHierarchicalInstancedStaticMesh _ashism_for_spiral) _array_index 2 (.Z (Math|Vector|BreakVector (Utilities|Array|Get(acopy) _colours _array_index))) true)
    (Components|InstancedStaticMesh|SetCustomDataValue (Variables|/Game/KitchenMishapSpiral/Blueprints/HismForSpiral.HismForSpiral_C|GetHierarchicalInstancedStaticMesh _ashism_for_spiral) _array_index 3 (Utilities|Array|Get(acopy) _opacities _array_index) true)))

(fn ReloadSpiralTransforms
  (bind _ashism_for_spiral (Utilities|Casting|CastToHismForSpiral (Variables|/Script/Engine.ChildActorComponent|GetChildActor (Variables|Default|GetExampleDaySpiral))))
  (bind _ashism_for_spiral_2 (Utilities|Casting|CastToHismForSpiral (Variables|/Script/Engine.ChildActorComponent|GetChildActor (Variables|Default|GetExampleDaySpiral1))))
  (bind (_colours _opacities _hism2transforms _returnvalue) (CallFunction|BuildRenderedJson "0.000000,0.000000,50.000000" 1e+02 (Variables|Default|GetJsonPath) (Variables|Default|GetMaxAssets)))
  (Class|InstancedStaticMeshComponent|BatchUpdateInstancesTransforms (Variables|/Game/KitchenMishapSpiral/Blueprints/HismForSpiral.HismForSpiral_C|GetHierarchicalInstancedStaticMesh _ashism_for_spiral) 0 _returnvalue false true true)
  (Class|InstancedStaticMeshComponent|BatchUpdateInstancesTransforms (Variables|/Game/KitchenMishapSpiral/Blueprints/HismForSpiral.HismForSpiral_C|GetHierarchicalInstancedStaticMesh _ashism_for_spiral_2) 0 _hism2transforms false true true))